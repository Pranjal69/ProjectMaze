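; Locked door actor for a maze game that the player opens by spending a key.
; A trigger volume enables the door's input only while the player overlaps it, and Interact consumes one of the character's keys and refreshes the HUD through the game mode.
; A key mesh is then spawned at runtime on the keyhole, a sound plays, and one timeline animates both key and door.
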(event `self.TriggerVolum.OnComponentBeginOverlap`
  (params (OverlappedComponent :type "PrimitiveComponent Object Reference") (OtherActor :type "Actor Object Reference") (OtherComp :type "PrimitiveComponent Object Reference") (OtherBodyIndex :type Integer) (bFromSweep :type Boolean) (SweepResult :type "HitResult Structure (by ref)"))
  (if (== OtherActor (`GameplayStatics.GetPlayerCharacter` 0))
    (`self.EnableInput` (`GameplayStatics.GetPlayerController` 0))))

(event `InputAction|Interact`
  (params (Key :type "Key Structure"))
  (:`Pressed`
    (bind _asgame_character (cast `/Game/Player/GameCharacter` (`GameplayStatics.GetPlayerCharacter` 0)))
    (bind _numberofkeys (`/Game/Player/GameCharacter.NumberOfKeys` _asgame_character))
    (if (> _numberofkeys 0)
      (`/Engine/EditorBlueprintResources/StandardMacros.DecrementInt` _numberofkeys
        (:`  `
          (bind _asmaze_game_mode (cast `/Game/GameSettings/MazeGameMode` (`GameplayStatics.GetGameMode`)))
          (`/Game/UI/HeadsUpEditor.UpdateSkulls` (`/Game/GameSettings/MazeGameMode.HeadsUpDisplay` _asmaze_game_mode))
          (bind _returnvalue (`AddComponent|NODE_AddStaticMeshComponent-0`))
          (bind _output_get (set `self.KeyMesh` _returnvalue))
          (`SceneComponent.K2_AttachToComponent` _output_get (`self.Keyhole`) "None" "SnapToTarget" "SnapToTarget" "SnapToTarget" true)
          (`GameplayStatics.PlaySoundAtLocation` "/Game/Music/DoorOpening_SFX.DoorOpening_SFX" (`self.K2_GetActorLocation`) (struct) 1.0 1.0 0.0 null null null)
          (bind (_direction _doorposition _keyposition) (`Timeline|Timeline_0` :!via `PlayFromStart`)
            (:`Update`
              (`SceneComponent.K2_SetRelativeLocation` (`self.KeyMesh`) (`KismetMathLibrary.MakeVector` 0.0 _keyposition) false false)
              (`SceneComponent.K2_SetRelativeLocation` (`self.Door`) (`KismetMathLibrary.MakeVector` 0.0 0.0 _doorposition) false false))))))))

(event `self.TriggerVolum.OnComponentEndOverlap`
  (params (OverlappedComponent :type "PrimitiveComponent Object Reference") (OtherActor :type "Actor Object Reference") (OtherComp :type "PrimitiveComponent Object Reference") (OtherBodyIndex :type Integer))
  (if (== OtherActor (`GameplayStatics.GetPlayerCharacter` 0))
    (`self.DisableInput` (`GameplayStatics.GetPlayerController` 0))))

(fn `UserConstructionScript`)