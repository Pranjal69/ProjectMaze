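; KeyPlatform is a pickup actor in the maze game that lets the player collect a key, shown as a skull on the HUD.
; Its trigger volume enables input while the player overlaps it and disables it on exit.
; Pressing Interact destroys the Key component if still valid, increments the character's key count, refreshes the HUD skulls through MazeGameMode, and plays a pickup sound.
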(event `self.TriggerVolume.OnComponentBeginOverlap`
  (params (OverlappedComponent :type "PrimitiveComponent Object Reference") (OtherActor :type "Actor Object Reference") (OtherComp :type "PrimitiveComponent Object Reference") (OtherBodyIndex :type Integer) (bFromSweep :type Boolean) (SweepResult :type "HitResult Structure (by ref)"))
  (if (== OtherActor (`GameplayStatics.GetPlayerCharacter` 0))
    (`self.EnableInput` (`GameplayStatics.GetPlayerController` 0))))

(event `InputAction|Interact`
  (params (Key :type "Key Structure"))
  (:`Pressed`
    (`/Engine/EditorBlueprintResources/StandardMacros.IsValid` (`self.Key`)
      (:`Is Valid`
        (`ActorComponent.K2_DestroyComponent` (`self.Key`))
        (bind _asgame_character (cast `/Game/Player/GameCharacter` (`GameplayStatics.GetPlayerCharacter` 0)))
        (`/Engine/EditorBlueprintResources/StandardMacros.IncrementInt` (`/Game/Player/GameCharacter.NumberOfKeys` _asgame_character)
          (:`  `
            (bind _asmaze_game_mode (cast `/Game/GameSettings/MazeGameMode` (`GameplayStatics.GetGameMode`)))
            (`/Game/UI/HeadsUpEditor.UpdateSkulls` (`/Game/GameSettings/MazeGameMode.HeadsUpDisplay` _asmaze_game_mode))
            (`GameplayStatics.PlaySoundAtLocation` "/Game/Music/PickupSkull_SFX.PickupSkull_SFX" (`self.K2_GetActorLocation` (`GameplayStatics.GetPlayerCharacter` 0)) (struct) 1.0 1.0 0.0 null null null)))))))

(event `self.TriggerVolume.OnComponentEndOverlap`
  (params (OverlappedComponent :type "PrimitiveComponent Object Reference") (OtherActor :type "Actor Object Reference") (OtherComp :type "PrimitiveComponent Object Reference") (OtherBodyIndex :type Integer))
  (if (== OtherActor (`GameplayStatics.GetPlayerCharacter` 0))
    (`self.DisableInput` (`GameplayStatics.GetPlayerController` 0))))

(fn `UserConstructionScript`)